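; Climbable ladder for the Knight, built in the Construction Script from repeated meshes with configurable count, spacing and trigger transforms.
; Hold snaps the character to the ladder and switches to Flying with the climbing flag set; Unhold restores Walking.
; Top overlap while climbing plays a montage whose notify moves the capsule up and forward and restores Walking, guarded by a DoOnce.
; Bottom overlap only records a flag.
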(event `/Game/Game/Actor/Ladder/BPI_HoldableObject.Hold`
  (params (Character :type "Character Object Reference"))
  (`self.HandleInteraction` Character))

(event `/Game/Game/Actor/Ladder/BPI_HoldableObject.Unhold`
  (params (Character :type "Character Object Reference"))
  (bind _asknight (cast `/Game/Game/Character/Knight` Character))
  (bind _charactermovement (`Character.CharacterMovement` _asknight))
  (`CharacterMovementComponent.SetMovementMode` _charactermovement "MOVE_Walking" 0)
  (set `/Game/Game/Character/Knight.IsClimbingLadder` false _asknight)
  (set `CharacterMovementComponent.bOrientRotationToMovement` true _charactermovement))

(event `self.TopCollision.OnComponentBeginOverlap`
  (params (OverlappedComponent :type "PrimitiveComponent Object Reference") (OtherActor :type "Actor Object Reference") (OtherComp :type "PrimitiveComponent Object Reference") (OtherBodyIndex :type Integer) (bFromSweep :type Boolean) (SweepResult :type "HitResult Structure (by ref)"))
  (bind _asknight (cast `/Game/Game/Character/Knight` OtherActor))
  (if (`/Game/Game/Character/Knight.IsClimbingLadder` _asknight)
    (`/Engine/EditorBlueprintResources/StandardMacros.DoOnce` false :!label _label
      (:`Completed`
        (`|PlayMontage` (`Character.Mesh` _asknight) "/Game/Game/Character/RM_Animation/Climb/RM_Climbing2_Montage.RM_Climbing2_Montage"
          (:`OnNotifyBegin`
            (set `/Game/Game/Character/Knight.IsClimbingLadder` false _asknight)
            (bind (_returnvalue_x _returnvalue_y _returnvalue_z) (`KismetMathLibrary.BreakVector` (`SceneComponent.K2_GetComponentLocation` (`Character.CapsuleComponent` _asknight))))
            (bind _returnvalue (`self.GetActorForwardVector` _asknight))
            (`KismetSystemLibrary.MoveComponentTo` (`Character.CapsuleComponent` _asknight) (+ (`KismetMathLibrary.MakeVector` _returnvalue_x _returnvalue_y (+ _returnvalue_z 80.0)) (* _returnvalue 45.0)) (`KismetMathLibrary.MakeRotFromX` _returnvalue) false false 0.3)
            (bind _charactermovement (`Character.CharacterMovement` _asknight))
            (`CharacterMovementComponent.SetMovementMode` _charactermovement "MOVE_Walking" 0)
            (set `CharacterMovementComponent.bOrientRotationToMovement` true _charactermovement)
            (`self.종료`)))))))

(event `종료`
  (goto _label :!via `Reset`))

(event `self.BottomCollision.OnComponentBeginOverlap`
  (params (OverlappedComponent :type "PrimitiveComponent Object Reference") (OtherActor :type "Actor Object Reference") (OtherComp :type "PrimitiveComponent Object Reference") (OtherBodyIndex :type Integer) (bFromSweep :type Boolean) (SweepResult :type "HitResult Structure (by ref)"))
  (cast `/Game/Game/Character/Knight` OtherActor)
  (set `self.BottomCollisionOverlap` true))

(event `self.BottomCollision.OnComponentEndOverlap`
  (params (OverlappedComponent :type "PrimitiveComponent Object Reference") (OtherActor :type "Actor Object Reference") (OtherComp :type "PrimitiveComponent Object Reference") (OtherBodyIndex :type Integer))
  (cast `/Game/Game/Character/Knight` OtherActor)
  (set `self.BottomCollisionOverlap` false))

(fn `HandleInteraction`
  (params (Character :type "Character Object Reference"))
  (bind (_returnvalue_location _returnvalue_rotation _returnvalue_scale) (`KismetMathLibrary.BreakTransform` (`self.GetTransform` Character)))
  (bind (_returnvalue_roll _returnvalue_pitch _returnvalue_yaw) (`KismetMathLibrary.BreakRotator` (`self.K2_GetActorRotation`)))
  (bind _character (`local.Character`))
  (bind (_returnvalue_x _returnvalue_y _returnvalue_z) (`KismetMathLibrary.BreakVector` (`self.K2_GetActorLocation` (`local.Character`))))
  (bind _charactermovement (`Character.CharacterMovement` _character))
  (`/Engine/EditorBlueprintResources/StandardMacros.IsValid` Character
    (:`Is Valid`
      (bind _output_get (set `self.CharacterNewTransformLocation` (`KismetMathLibrary.MakeTransform` (`KismetMathLibrary.MakeVector` (.x (+ (`self.K2_GetActorLocation`) (* (`self.GetActorRightVector`) -48.0))) (.y (+ (`self.K2_GetActorLocation`) (* (`self.GetActorRightVector`) -48.0))) _returnvalue_z) (`KismetMathLibrary.MakeRotator` _returnvalue_roll _returnvalue_pitch (+ _returnvalue_yaw 90.0)) _returnvalue_scale)))
      (`self.K2_SetActorTransform` _character _output_get true false)
      (`CharacterMovementComponent.SetMovementMode` _charactermovement "MOVE_Flying" 0)
      (set `/Game/Game/Character/Knight.IsClimbingLadder` true (cast `/Game/Game/Character/Knight` _character :!pure true))
      (set `CharacterMovementComponent.bOrientRotationToMovement` false _charactermovement)
      (`MovementComponent.StopMovementImmediately` _charactermovement))))

(fn `UserConstructionScript`
  (locals (StaticMesh :type "StaticMeshComponent Object Reference"))
  (for _index (range (`self.LadderCount`))
    (bind _returnvalue (`AddComponent|NODE_AddStaticMeshComponent-0` :`RelativeTransform` (`KismetMathLibrary.MakeTransform` (`KismetMathLibrary.MakeVector` 0.0 0.0 (* _index (`self.DistanceBetweenLadder`))) (struct) (0.2 0.2 0.2))))
    (bind _output_get (set `local.StaticMesh` _returnvalue))
    (`StaticMeshComponent.SetStaticMesh` _output_get (`self.LadderMesh`))
    (`PrimitiveComponent.SetCollisionEnabled` (`local.StaticMesh`) "NoCollision"))
  (`SceneComponent.K2_SetRelativeTransform` (`self.LadderCollision`) (`self.LadderCollisionTransform`) false false)
  (`SceneComponent.K2_SetRelativeTransform` (`self.TopCollision`) (`self.TopCollisionTransform`) false false))